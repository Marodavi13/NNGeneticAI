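; Neural network manager for a genetic driving simulation, handling the on-screen network display and the return of the specimen pawn to its start.
; On BeginPlay it binds to the simulation-started event, which creates and initializes the W_NeuralNetwork viewport widget.
; MovePawntoTargetPoint uses a Timeline to lerp the pawn to StartingPoint without sweep, then zeroes its velocity; an author note says the Timeline prevents runaway movement.
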(event `self.ReceiveBeginPlay`
  (set `GeneticAIGameModeBase.Manager` null (`GeneticFL.GetGeneticGameMode` self))
  (add `self.OnSimulationStarted` (delegate `OnSimulationStartedEvent`)))

(event `OnSimulationStartedEvent`
  (bind _returnvalue (`|CreateWidget` "/Game/Content/Widgets/W_NeuralNetwork.W_NeuralNetwork_C"))
  (bind _output_get (set `self.Widget` _returnvalue))
  (`UserWidget.AddToViewport` _output_get 0)
  (`NeuralNetworkWidget.InitWidget` _returnvalue))

(event `self.MovePawnToTargetPoint`
  (bind _specimenpawn (`self.SpecimenPawn`))
  ;[1 1 1] Use this Timeline or Bob goes to infinite
  (bind _output_get (set `self.LastLocation` (`self.K2_GetActorLocation` _specimenpawn)))
  (bind (_direction _newtrack_0) (`Timeline|Timeline_0` :!via `PlayFromStart`)
    (:`Update`
      (`self.K2_SetActorLocation` _specimenpawn (`KismetMathLibrary.VLerp` _output_get (`self.K2_GetActorLocation` (`self.StartingPoint`)) _newtrack_0) false false))
    (:`Finished`
      (set `MovementComponent.Velocity` (0.0 0.0 0.0) (`self.SpecimenPawnMovement`)))))

(fn `UserConstructionScript`)