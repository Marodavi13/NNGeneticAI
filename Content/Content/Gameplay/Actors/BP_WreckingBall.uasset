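; Wrecking ball actor that acts as a sensing agent in a neural network simulation run over successive specimens.
; Manager events enable its query-only sphere collision for each new specimen and disable it when a run ends.
; Each tick, forward, left and right line traces fill three values for NeuralInput.
; Forward and left hits give normalized distances, right hits always give zero, and misses give the raw maximum distance.
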(event `self.ReceiveBeginPlay`
  (bind _manager (`self.Manager`))
  (bind _outactors (`GameplayStatics.GetAllActorsOfClass` "/Script/GeneticAI.DrivingLane"))
  (set `self.DrivingLine` (`|GetArrayItem` _outactors))
  (add `NeuralNetworkManager.OnNewSpecimen` _manager (delegate `EnableCollision`))
  (add `NeuralNetworkManager.OnRunEnded` _manager (delegate `DisableCollision`)))

(event `EnableCollision`
  (params (NewSpecimenIndex :type Byte))
  (`PrimitiveComponent.SetCollisionEnabled` (`self.SphereCollision`) "QueryOnly"))

(event `DisableCollision`
  (params (TimeUntilNextSimulation :type "Float (double-precision)") (Fitness :type "Float (double-precision)") (NumberOfSpecimen :type Byte))
  (`PrimitiveComponent.SetCollisionEnabled` (`self.SphereCollision`) "NoCollision"))

(event `self.ReceiveTick`
  (params (DeltaSeconds :type "Float (single-precision)"))
  (bind _returnvalue (`self.K2_GetActorLocation`))
  (bind _returnvalue_2 (`self.K2_GetActorLocation`))
  (bind _returnvalue_3 (`self.K2_GetActorLocation`))
  (bind _inputvalues (`self.InputValues`))
  (bind _maxforwarddistance (`self.MaxForwardDistance`))
  (bind _maxsidedistance (`self.MaxSideDistance`))
  (bind _inputvalues_2 (`self.InputValues`))
  (bind _maxsidedistance_2 (`self.MaxSideDistance`))
  (bind _inputvalues_3 (`self.InputValues`))
  ;[1 1 1] Placeholder
  (bind (_outhit _returnvalue_4) (`KismetSystemLibrary.LineTraceSingle` :`Start` _returnvalue_3 :`End` (+ _returnvalue_3 (* (`self.GetActorForwardVector`) (`self.MaxForwardDistance`))) :`TraceChannel` "TraceTypeQuery1" :`DrawDebugType` "ForOneFrame"))
  (if _returnvalue_4
    (`KismetArrayLibrary.Array_Set` _inputvalues 0 (/ (`.Distance` (`GameplayStatics.BreakHitResult` _outhit)) _maxforwarddistance))
    (else
      (`KismetArrayLibrary.Array_Set` _inputvalues 0 _maxforwarddistance)))
  (bind (_outhit_2 _returnvalue_5) (`KismetSystemLibrary.LineTraceSingle` :`Start` _returnvalue :`End` (+ _returnvalue (* (`self.GetActorRightVector`) (- 0.0 (`self.MaxSideDistance`)))) :`TraceChannel` "TraceTypeQuery1" :`DrawDebugType` "ForOneFrame"))
  (if _returnvalue_5
    (`KismetArrayLibrary.Array_Set` _inputvalues_2 1 (/ (`.Distance` (`GameplayStatics.BreakHitResult` _outhit_2)) _maxsidedistance))
    (else
      (`KismetArrayLibrary.Array_Set` _inputvalues_2 1 _maxsidedistance)))
  (bind (_outhit_3 _returnvalue_6) (`KismetSystemLibrary.LineTraceSingle` :`Start` _returnvalue_2 :`End` (+ _returnvalue_2 (* (`self.GetActorRightVector`) (`self.MaxSideDistance`))) :`TraceChannel` "TraceTypeQuery1" :`DrawDebugType` "ForOneFrame"))
  (if _returnvalue_6
    (`KismetArrayLibrary.Array_Set` _inputvalues_3 2 (/ 0.0 _maxsidedistance_2))
    (else
      (`KismetArrayLibrary.Array_Set` _inputvalues_3 2 _maxsidedistance_2)))
  (`NeuralInputComponent.SetInputs` (`self.NeuralInput`) (`self.InputValues`)))

(fn `UserConstructionScript`
  (`KismetArrayLibrary.Array_Resize` (`self.InputValues`) 3))