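; Player controller for the wrecking ball pawn in a genetic-algorithm simulation.
; On BeginPlay it caches the controlled pawn as a BP_WreckingBall.
; K ends the current specimen simulation through the genetic game mode's manager.
; W, A and D update forward and turn values, but Tick is empty and the calls passing them to the ball are disconnected, so they never move it.
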(event `self.ReceiveBeginPlay`
  (bind _asbp_wrecking_ball (cast `/Game/Content/Gameplay/Actors/BP_WreckingBall` (`self.K2_GetPawn`)))
  (set `self.Ball` _asbp_wrecking_ball))

(event `Key|K`
  (params (Key :type "Key Structure"))
  (bind _manager (`GeneticAIGameModeBase.Manager` (`GeneticFL.GetGeneticGameMode` self)))
  (:`Pressed`
    (`/Engine/EditorBlueprintResources/StandardMacros.IsValid` _manager
      (:`Is Valid`
        (`NeuralNetworkManager.EndSpecimenSimulation` _manager)))))

(event `Key|W`
  (params (Key :type "Key Structure"))
  (:`Pressed`
    (set `self.ValueX` 1.0))
  (:`Released`
    (set `self.ValueX` 0.0)))

(event `Key|A`
  (params (Key :type "Key Structure"))
  (bind _valuey (`self.ValueY`))
  (:`Pressed`
    (`/Engine/EditorBlueprintResources/StandardMacros.DecrementFloat` _valuey :!label _label))
  (:`Released`
    (`/Engine/EditorBlueprintResources/StandardMacros.IncrementFloat` _valuey :!label _label_2)))

(event `Key|D`
  (params (Key :type "Key Structure"))
  (:`Pressed`
    (goto _label_2))
  (:`Released`
    (goto _label)))

(event `self.ReceiveTick`
  (params (DeltaSeconds :type "Float (single-precision)")))

(fn `UserConstructionScript`)