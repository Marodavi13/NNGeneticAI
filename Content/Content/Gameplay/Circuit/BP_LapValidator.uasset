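; A trigger-box actor on the circuit that gates lap counting for the driving neural network training.
; On BeginPlay, after a one-tick delay, it caches the DrivingNeuralNetworkManager from the genetic game mode.
; When a WreckingBall overlaps its box, it sets the manager's IsIncreaseLapAllowed flag to its EnableLap value, so each placed instance either allows or blocks lap increments.
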(event `self.ReceiveBeginPlay`
  (`KismetSystemLibrary.Delay` 0.0)
  (bind _asdriving_neural_network_manager (cast `DrivingNeuralNetworkManager` (`GeneticAIGameModeBase.Manager` (`GeneticFL.GetGeneticGameMode` self))))
  (set `self.Manager` _asdriving_neural_network_manager))

(event `self.Box.OnComponentBeginOverlap`
  (params (OverlappedComponent :type "PrimitiveComponent Object Reference") (OtherActor :type "Actor Object Reference") (OtherComp :type "PrimitiveComponent Object Reference") (OtherBodyIndex :type Integer) (bFromSweep :type Boolean) (SweepResult :type "HitResult Structure (by ref)"))
  (if (`KismetMathLibrary.ClassIsChildOf` (`GameplayStatics.GetObjectClass` OtherActor) "/Script/GeneticAI.WreckingBall")
    (set `DrivingNeuralNetworkManager.bIsIncreaseLapAllowed` (`self.bEnableLap`) (`self.Manager`))))

(fn `UserConstructionScript`)